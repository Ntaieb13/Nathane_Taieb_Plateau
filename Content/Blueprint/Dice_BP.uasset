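; Dice actor for a board game that rolls itself every 8 seconds and triggers pawn moves.
; Each roll teleports it to a fixed elevated spot with random rotation, then polls its location every 0.2 seconds until unchanged.
; The face whose arrow component points up sets DiceResult.
; A FlipFlop then alternates PionNumberInt between two pawns before calling the PionMove dispatcher.
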(event Custom|Stop
  ;[1 1 1] verifier si le dés est arréter
  (Variables|Default|SetActor_Loc (Transformation|GetActorLocation))
  (Utilities|FlowControl|Delay 0.2)
  (if (Utilities|Operators|EqualEqual (Variables|Default|GetActor_Loc) (Transformation|GetActorLocation) 0.0)
    (CallFunction|Result)
    (else
      (CallFunction|Stop))))

(event Custom|Result
  ;[1 1 1] resulta du dé en fonction de la surface
  (if (Utilities|Operators|EqualEqual (Math|Vector|GetForwardVector (Variables|Default|GetArrow1)) "0.000000,0.000000,1.000000" 0.5)
    (Development|PrintString "1" true true "(R=0.000000,G=0.660000,B=1.000000,A=1.000000)" 5.0)
    (Variables|Default|SetDice%20Result 1)
    (Utilities|FlowControl|FlipFlop :!label _label
      (:A
        (Variables|Default|SetPion_Number_Int 0))
      (:B
        (Variables|Default|SetPion_Number_Int 1)))
    (Default|CallPionMoveDispacher)
    (elif (Utilities|Operators|EqualEqual (Math|Vector|GetForwardVector (Variables|Default|GetArrow2)) "0.000000,0.000000,1.000000" 0.5)
      (Development|PrintString "2" true true "(R=0.000000,G=0.660000,B=1.000000,A=1.000000)" 5.0)
      (Variables|Default|SetDice%20Result 2)
      (goto _label)
      (elif (Utilities|Operators|EqualEqual (Math|Vector|GetForwardVector (Variables|Default|GetArrow3)) "0.000000,0.000000,1.000000" 0.5)
        (Development|PrintString "3" true true "(R=0.000000,G=0.660000,B=1.000000,A=1.000000)" 5.0)
        (Variables|Default|SetDice%20Result 3)
        (goto _label)
        (elif (Utilities|Operators|EqualEqual (Math|Vector|GetForwardVector (Variables|Default|GetArrow4)) "0.000000,0.000000,1.000000" 0.5)
          (Development|PrintString "4" true true "(R=0.000000,G=0.660000,B=1.000000,A=1.000000)" 5.0)
          (Variables|Default|SetDice%20Result 4)
          (goto _label)
          (elif (Utilities|Operators|EqualEqual (Math|Vector|GetForwardVector (Variables|Default|GetArrow5)) "0.000000,0.000000,1.000000" 0.5)
            (Development|PrintString "5" true true "(R=0.000000,G=0.660000,B=1.000000,A=1.000000)" 5.0)
            (Variables|Default|SetDice%20Result 5)
            (goto _label)
            (elif (Utilities|Operators|EqualEqual (Math|Vector|GetForwardVector (Variables|Default|GetArrow6)) "0.000000,0.000000,1.000000" 0.5)
              (Development|PrintString "6" true true "(R=0.000000,G=0.660000,B=1.000000,A=1.000000)" 5.0)
              (Variables|Default|SetDice%20Result 6)
              (goto _label))))))))

(event Custom|Rolling
  (bind _returnvalue (Math|Random|RandomFloatinRange 0.0 3.6e+02))
  ;[1 1 1] faire rouler le dé*
  (Transformation|SetActorLocation "90.000000,-130.000000,980.000000" false false)
  (Transformation|SetActorRotation (Math|Rotator|MakeRotator _returnvalue _returnvalue _returnvalue))
  (CallFunction|Stop)
  (Utilities|FlowControl|Delay 8.0)
  (CallFunction|Rolling))

(event EventBeginPlay
  (CallFunction|Rolling))

(fn ConstructionScript)