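; PB_Dice is an Actor Blueprint that simulates a dice roll when play begins.
; RollDice resets ActualDiceResult, then loops from 0 to DiceNumber, adding a random integer between 1 and DiceType on each pass.
; The total stays in ActualDiceResult, and nothing in these graphs displays or passes it on.
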(event EventBeginPlay
  (CallFunction|RollDice))

(event Collision|EventActorBeginOverlap
  (params (OtherActor :type Actor%20Object%20Reference)))

(event EventTick
  (params (DeltaSeconds :type Float%20%28single-precision%29)))

(fn ConstructionScript)

(fn RollDice
  (Variables|Default|SetActualDiceResult 0)
  (for _index (range 0 (Variables|Default|GetDiceNumber))
    (bind _output_get (Variables|Default|SetActualDiceResult (+ (Variables|Default|GetActualDiceResult) (Math|Random|RandomIntegerinRange 1 (Variables|Default|GetDiceType)))))))